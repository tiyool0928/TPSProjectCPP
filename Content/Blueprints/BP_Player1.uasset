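; Player Blueprint that creates the UI_Screen HUD and drives its health and weapon display.
; BeginPlay adds the widget to the viewport, then after a short delay refreshes HP and selects the non-grenade state.
; OnUsingGrenade passes the grenade flag to the widget and calls SwapWeapon.
; UIctrlHP writes the current/initial HP text and computes HpRatio with modulo rather than division, so full health yields zero.
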(event `self.ReceiveBeginPlay`
  (bind _returnvalue (`|CreateWidget` "/Game/Blueprints/UI/UI_Screen.UI_Screen_C" (`GameplayStatics.GetPlayerController` 0)))
  (bind _output_get (set `self.UI_Screen` _returnvalue))
  (`UserWidget.AddToViewport` _output_get 0)
  (`KismetSystemLibrary.Delay` 0.05)
  (`self.UIctrlHP`)
  (`self.OnUsingGrenade` false))

(event `self.OnUsingGrenade`
  (params (isGrenade :type Boolean))
  (bind _ui_screen (`self.UI_Screen`))
  (`/Engine/EditorBlueprintResources/StandardMacros.IsValid` _ui_screen
    (:`Is Valid`
      (set `/Game/Blueprints/UI/UI_Screen.isGrenaded` isGrenade _ui_screen)
      (`/Game/Blueprints/UI/UI_Screen.SwapWeapon` _ui_screen))))

(fn `UIctrlHP`
  (set `/Game/Blueprints/UI/UI_Screen.hpRatio` (mod (`KismetMathLibrary.Conv_IntToDouble` (`self.hp`)) (`KismetMathLibrary.Conv_IntToDouble` (`self.initialHp`))) (`self.UI_Screen`))
  (set `/Game/Blueprints/UI/UI_Screen.hpString` (`KismetStringLibrary.Concat_StrStr` (`KismetStringLibrary.Conv_IntToString` (`self.hp`)) "/" (`KismetStringLibrary.Conv_IntToString` (`self.initialHp`))) (`self.UI_Screen`)))

(fn `UserConstructionScript`)